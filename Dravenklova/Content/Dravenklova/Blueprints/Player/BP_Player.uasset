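; Player Blueprint that animates the body procedurally from look direction and interaction.
; On BeginPlay it updates its attributes; each Tick the head follows control pitch and the torso eases toward the head's world rotation through a frame-time-scaled lerp from its previous rotation.
; Interact begin and end events play and reverse a timeline that blends the right arm between a rest pose and a use pose.
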(event EventTick
  (params (DeltaSeconds :type Float%20%28single-precision%29))
  (bind _torso (Variables|Default|GetTorso))
  (|CallParentFunction DeltaSeconds)
  (Transformation|SetRelativeRotation (Variables|Default|GetHead) (Math|Rotator|MakeRotator 0.0 (.Pitch (Math|Rotator|BreakRotator (Pawn|GetControlRotation :!class /Script/Engine.Pawn))) 0.0) false false)
  (Transformation|SetWorldRotation _torso (Math|Rotator|Lerp(Rotator) (Variables|Default|GetLastTorsoRotation) (Transformation|GetWorldRotation (Variables|Default|GetHead)) (* DeltaSeconds 1e+01) true) false false)
  (Variables|Default|SetLastTorsoRotation (Transformation|GetWorldRotation _torso)))

(event EventProvideInteractEnd
  (params (Reciever :type Actor%20Object%20Reference))
  (bind _armstuff (Timeline|ArmUse Reverse)
    (:Update
      (Transformation|SetRelativeLocationAndRotation (Variables|Default|GetArmRight) (Math|Vector|Lerp(Vector) "30.000000,30.000000, 0" "40.000000,30.000000,5.000000" _armstuff) (Math|Rotator|Lerp(Rotator) "0,-90.000000, 0" "60.000000,-100.000000,10.000000" _armstuff) false false))))

(event EventBeginPlay
  (Class|DAttributes|UpdateAttributes (Variables|Default|Getm_Attributes)))

(event EventProvideInteractBegin
  (params (Reciever :type Actor%20Object%20Reference))
  (bind _armstuff (Timeline|ArmUse Play)
    (:Update
      (Transformation|SetRelativeLocationAndRotation (Variables|Default|GetArmRight) (Math|Vector|Lerp(Vector) "30.000000,30.000000, 0" "40.000000,30.000000,5.000000" _armstuff) (Math|Rotator|Lerp(Rotator) "0,-90.000000, 0" "60.000000,-100.000000,10.000000" _armstuff) false false))))

(fn ConstructionScript
  (|CallParentFunction))