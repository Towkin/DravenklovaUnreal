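; BP_NoteBase is a base world-item note that lifts up in front of the interacting user's view and returns to its spawn transform afterwards.
; Tick computes a hold transform 100 units along the user's view, rotated to face them.
; A timeline lerps from the spawn transform to it; once forward playback finishes, the note follows the view.
; Ending interaction clears the user and reverses the timeline.
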(event EventTick
  (params (DeltaSeconds :type Float%20%28single-precision%29))
  (bind _currentuser (Variables|Default|GetCurrentUser))
  (bind (_outlocation _outrotation) (Actor|GetActorEyesViewPoint _currentuser))
  (bind (_roll _pitch _yaw) (Math|Rotator|BreakRotator _outrotation))
  (if (!= (Variables|Default|GetCurrentUser) 0)
    (bind _output_get (Variables|Default|SetHoldTransform (Math|Transform|MakeTransform (+ _outlocation (* (Math|Vector|GetForwardVector _outrotation) 1e+02)) (Math|Rotator|MakeRotator 0.0 (- (* _pitch -1.0) 9e+01) (+ _yaw 1.8e+02)))))
    (if (Variables|Default|GetHolding)
      (Transformation|SetActorTransform _output_get false true))))

(event EventInteractBegin
  (params (User :type D%20Character%20Object%20Reference))
  (Variables|Default|SetCurrentUser User)
  (bind (_direction _notelerp) (Timeline|NoteTimeline Play)
    (:Update
      (Transformation|SetActorTransform (Math|Transform|Lerp(Transform) (Variables|Default|GetSpawnLocation) (Variables|Default|GetHoldTransform) _notelerp) false true))
    (:Finished
      (switch Utilities|FlowControl|Switch|SwitchonETimelineDirection _direction
        (:Forward
          (Variables|Default|SetHolding true))))))

(event EventBeginPlay
  (Variables|Default|SetSpawnLocation (Transformation|GetActorTransform)))

(event EventInteractEnd
  (params (User :type D%20Character%20Object%20Reference))
  (Variables|Default|SetHolding false)
  (Variables|Default|SetCurrentUser 0)
  (bind (_direction _notelerp) (Timeline|NoteTimeline Reverse)
    (:Update
      (Transformation|SetActorTransform (Math|Transform|Lerp(Transform) (Variables|Default|GetSpawnLocation) (Variables|Default|GetHoldTransform) _notelerp) false true))
    (:Finished
      (switch Utilities|FlowControl|Switch|SwitchonETimelineDirection _direction
        (:Forward
          (Variables|Default|SetHolding true))))))

(fn ConstructionScript)