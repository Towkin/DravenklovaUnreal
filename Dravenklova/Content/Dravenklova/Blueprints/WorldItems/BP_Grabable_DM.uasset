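; Grabbable physics world item that a player can push with a short interaction or carry by holding it.
; Holding past PushTime adds a physics handle, and a short Delay loop eases it toward a point before the user's view with optional rotation offset and yaw-only alignment.
; Ending interaction destroys the handle, or applies a forward impulse if none exists yet.
; The user's HumorYellow attribute and the mesh's mass scale follow speed and push strength.
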(event EventInteractBegin
  (params (User :type D%20Character%20Object%20Reference))
  (bind _physicsmesh (Variables|Default|GetPhysicsMesh))
  (Variables|Grabable|SetUser User)
  (Utilities|FlowControl|Delay (Variables|Grabable|GetPushTime))
  (if (!= (Variables|Grabable|GetUser) 0)
    (bind _returnvalue (AddComponent|AddPhysicsHandleComponent))
    (bind _output_get (Variables|Default|SetHandle _returnvalue))
    (bind _returnvalue_2 (Physics|GetCenterOfMass _physicsmesh "None"))
    (Class|PrimitiveComponent|SetAngularDamping _physicsmesh (Variables|Grabable|GetRotDampeningGrabed))
    (Class|PhysicsHandleComponent|GrabComponent _output_get _physicsmesh "None" (select (Variables|Grabable|GetGrabCenter) _returnvalue_2 (+ (.OutLocation (Actor|GetActorEyesViewPoint (Variables|Grabable|GetUser))) (* (Math|Vector|GetForwardVector (.OutRotation (Actor|GetActorEyesViewPoint (Variables|Grabable|GetUser)))) (Variables|Grabable|GetGrabDistance)))) (Variables|Grabable|GetLockRotation))
    (Utilities|FlowControl|Delay 0.01 :!label _label)
    (if (and (!= (Variables|Grabable|GetUser) 0) (!= (Variables|Default|GetHandle) 0))
      (Class|PhysicsHandleComponent|SetTargetLocationandRotation (Variables|Default|GetHandle) (Math|Vector|Lerp(Vector) (.TargetLocation (Class|PhysicsHandleComponent|GetTargetLocationandRotation (Variables|Default|GetHandle))) (+ (.OutLocation (Actor|GetActorEyesViewPoint (Variables|Grabable|GetUser))) (* (Math|Vector|GetForwardVector (.OutRotation (Actor|GetActorEyesViewPoint (Variables|Grabable|GetUser)))) (Variables|Grabable|GetGrabDistance))) (Math|Float|Clamp(Float) (/ (Math|Float|Lerp 2.0 1e+01 (Class|DAttributes|GetHumorYellow (Variables|/Script/Dravenklova.DCharacter|Getm_Attributes (Variables|Grabable|GetUser)))) (Physics|GetMass (Variables|Default|GetPhysicsMesh))))) (Math|Rotator|Lerp(Rotator) (.TargetRotation (Class|PhysicsHandleComponent|GetTargetLocationandRotation (Variables|Default|GetHandle))) (Math|Rotator|CombineRotators (Variables|Grabable|GetRotationOffset) (select (Variables|Grabable|GetYawRotationOnly) (Math|Rotator|MakeRotator 0.0 0.0 (.Yaw (Math|Rotator|BreakRotator (.OutRotation (Actor|GetActorEyesViewPoint (Variables|Grabable|GetUser)))))) (.OutRotation (Actor|GetActorEyesViewPoint (Variables|Grabable|GetUser))))) (Math|Float|Clamp(Float) (/ (Math|Float|Lerp 2.0 1e+01 (Class|DAttributes|GetHumorYellow (Variables|/Script/Dravenklova.DCharacter|Getm_Attributes (Variables|Grabable|GetUser)))) (Physics|GetMass (Variables|Default|GetPhysicsMesh)))) true))
      (goto _label))))

(event EventInteractEnd
  (params (User :type D%20Character%20Object%20Reference))
  (bind _physicsmesh (Variables|Default|GetPhysicsMesh))
  (Class|PrimitiveComponent|SetAngularDamping _physicsmesh 0.0)
  (if (!= (Variables|Default|GetHandle) 0)
    (Components|DestroyComponent (Variables|Default|GetHandle))
    (Variables|Default|SetHandle 0)
    (Variables|Grabable|SetUser 0 :!label _label)
    (elif (!= (Variables|Grabable|GetUser) 0)
      (Physics|AddImpulseatLocation (Variables|Default|GetPhysicsMesh) (* (Math|Vector|GetForwardVector (.OutRotation (Actor|GetActorEyesViewPoint (Variables|Grabable|GetUser)))) (+ (Math|Float|Lerp 1.5e+03 3.5e+03 (Class|DAttributes|GetHumorYellow (Variables|/Script/Dravenklova.DCharacter|Getm_Attributes (Variables|Grabable|GetUser)))) (* (Math|Float|Lerp 5e+01 2.5e+02 (Class|DAttributes|GetHumorYellow (Variables|/Script/Dravenklova.DCharacter|Getm_Attributes (Variables|Grabable|GetUser)))) (Physics|GetMass _physicsmesh)))) (+ (.OutLocation (Actor|GetActorEyesViewPoint (Variables|Grabable|GetUser))) (* (Math|Vector|GetForwardVector (.OutRotation (Actor|GetActorEyesViewPoint (Variables|Grabable|GetUser)))) (Variables|Grabable|GetGrabDistance))) "None")
      (goto _label))))

(fn ConstructionScript)