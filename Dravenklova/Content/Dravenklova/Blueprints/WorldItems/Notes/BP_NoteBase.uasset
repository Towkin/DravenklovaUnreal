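; Base Blueprint for an interactable note that shows its text through a decal and lights up while in use.
; A canvas render target draws the word-wrapped NoteText, using channel colors for background and glyphs, and feeds a dynamic decal material as TextTexture.
; Interaction fades a point light in via timeline.
; Ending it reverses the fade and pushes the physics mesh along the user's view direction.
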(event Custom|TextCanvasUpdate
  (params (Canvas :type Canvas%20Object%20Reference) (Width :type Integer) (Height :type Integer))
  (Canvas|DrawTexture :self Canvas :ScreenPosition "(X=0.000000,Y=0.000000)" :ScreenSize (Math|Vector2D|MakeVector2D (Math|Conversions|ToFloat(Integer) Width) (Math|Conversions|ToFloat(Integer) Height)) :RenderColor "(R=1.000000,G=0.000000,B=0.000000,A=1.000000)" :BlendMode "BLEND_Opaque")
  (for _array_element (Utilities|String|ParseIntoArray (Utilities|String|TrimTrailing (Utilities|String|Trim (Utilities|String|ToString(Text) (Variables|Default|GetNoteText)))) " " false)
    (if (Utilities|Enum|Equal(Enum) (Variables|Default|GetTempRenderString) "")
      (Variables|Default|SetTempRenderString _array_element)
      (else
        (Variables|Default|SetTempRenderString (Utilities|String|Append (Variables|Default|GetTempRenderString) " " _array_element))))
    (bind _returnvalue (Class|Canvas|StrLen Canvas (Variables|Default|GetNoteTextFont) (Variables|Default|GetTempRenderString)))
    (if (> (.X (Math|Vector2D|BreakVector2D _returnvalue)) (Math|Conversions|ToFloat(Integer) (Variables|Default|GetTextCanvasWidth)))
      (Utilities|Array|Add (Variables|Default|GetRenderStrings) (Variables|Default|GetOldRenderString))
      (Variables|Default|SetTempRenderString _array_element)
      (else
        (Variables|Default|SetOldRenderString (Variables|Default|GetTempRenderString))
        (Variables|Default|SetLineHeight (.Y (Math|Vector2D|BreakVector2D _returnvalue))))))
  (Utilities|Array|Add (Variables|Default|GetRenderStrings) (Variables|Default|GetTempRenderString))
  (for (_array_element_2 _array_index) (Variables|Default|GetRenderStrings)
    (HUD|DrawText Canvas (Variables|Default|GetNoteTextFont) _array_element_2 (Math|Vector2D|MakeVector2D 0.0 (* _array_index (Variables|Default|GetLineHeight))) "(R=0.000000,G=1.000000,B=0.000000,A=1.000000)" 0.0 "(R=0.000000,G=0.000000,B=1.000000,A=1.000000)" "(X=1.000,Y=1.000)" false false false "(R=1.000000,G=1.000000,B=1.000000,A=1.000000)"))
  (Utilities|Array|Clear (Variables|Default|GetRenderStrings))
  (Variables|Default|SetTempRenderString "")
  (Variables|Default|SetOldRenderString ""))

(event EventInteractBegin
  (params (User :type D%20Character%20Object%20Reference))
  (bind _output_get (Variables|Default|SetCurrentUser User))
  (|CallParentFunction _output_get)
  (bind _notelerp (Timeline|NoteTimeline Play)
    (:Update
      (Rendering|Components|Light|SetIntensity (Variables|Default|GetPointLight) (Math|Float|Lerp 0.0 0.25 _notelerp)))))

(event EventBeginPlay
  (|CallParentFunction)
  (bind _returnvalue (CanvasRenderTarget2D|CreateCanvasRenderTarget2D "/Script/Engine.CanvasRenderTarget2D" (Variables|Default|GetTextCanvasWidth) (Variables|Default|GetTextCanvasHeight)))
  (bind _output_get (Variables|Default|SetTextCanvasTexture _returnvalue))
  (EventDispatchers|BindEventtoOnCanvasRenderTargetUpdate _output_get (delegate Custom|TextCanvasUpdate))
  (CallFunction|SetupTextMaterial))

(event EventInteractEnd
  (params (User :type D%20Character%20Object%20Reference))
  (bind (_outlocation _outrotation) (Actor|GetActorEyesViewPoint User))
  (Physics|AddImpulseatLocation (Variables|Default|GetPhysicsMesh) (* (Math|Vector|GetForwardVector _outrotation) 1.5e+02) _outlocation "None")
  (bind _output_get (Variables|Default|SetCurrentUser 0))
  (|CallParentFunction _output_get)
  (bind _notelerp (Timeline|NoteTimeline Reverse)
    (:Update
      (Rendering|Components|Light|SetIntensity (Variables|Default|GetPointLight) (Math|Float|Lerp 0.0 0.25 _notelerp)))))

(fn ConstructionScript)

(fn SetupTextMaterial
  (bind _textcanvastexture (Variables|Default|GetTextCanvasTexture))
  (if (!= (Variables|Default|GetTextBaseMaterial) 0)
    (bind _returnvalue (Rendering|Material|CreateDynamicMaterialInstance (Variables|Default|GetTextBaseMaterial) :!class /Script/Engine.KismetMaterialLibrary))
    (bind _output_get (Variables|Default|SetTextDynMaterial _returnvalue))
    (Rendering|Components|Decal|SetDecalMaterial (Variables|Default|GetDecal) _output_get)
    (Class|CanvasRenderTarget2D|UpdateResource _textcanvastexture)
    (Rendering|Material|SetTextureParameterValue (Variables|Default|GetTextDynMaterial) "TextTexture" _textcanvastexture)
    (else
      (Class|VisualLoggerKismetLibrary|LogText "No valid TextBaseMaterial" "Blueprint Log"))))