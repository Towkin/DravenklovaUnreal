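; BP_Block is a grid-based level block that places portals and walls from its MBlockData.
; SetupPortals adds a child actor per portal entry, clamped to the tile grid and yawed by direction, using the portal class if flagged or forced, otherwise the wall class.
; SpawnBlockComponents runs it.
; The construction script sizes the occupation grid and optionally previews portals, occupied tiles as meshes, and the surrounding bounds box.
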(event EventSpawnBlockComponents
  (CallFunction|SetupPortals))

(fn ConstructionScript
  (bind _m_blockdata (Variables|Default|Getm_BlockData))
  (bind _visualizeoccupation (Variables|Block|GetVisualizeOccupation))
  (bind _m_blockdata_2 (Variables|Default|Getm_BlockData))
  (bind _m_blockdata_3 (Variables|Default|Getm_BlockData))
  (bind (_tilecount _blocklocation _blockdirection _occupationgrid) (Utilities|Struct|BreakBlockData _m_blockdata))
  (bind (_portalarray _tilecount_2 _tilesize _blocklocation_2 _blockdirection_2 _occupationgrid_2) (Utilities|Struct|BreakBlockData _m_blockdata_3))
  (bind (_tilecount_3 _tilesize_2) (Utilities|Struct|BreakBlockData _m_blockdata_2))
  (bind (_x _y _z) (Utilities|Struct|BreakIntVector _tilecount_3))
  (bind (_x_2 _y_2 _z_2) (Utilities|Struct|BreakIntVector _tilecount))
  (Utilities|FlowControl|Sequence
    (:then_0
      (Utilities|Array|Resize _occupationgrid (* _x_2 _y_2 _z_2)))
    (:then_1
      (if (Variables|Block|GetVisualizePortals)
        (CallFunction|SetupPortals)))
    (:then_2
      (Rendering|SetVisibility (Variables|Default|GetSurroundBox) _visualizeoccupation false)
      (if _visualizeoccupation
        (Utilities|FlowControl|Sequence
          (:then_0
            (for (_array_element _array_index) _occupationgrid_2
              (if _array_element
                (AddComponent|AddStaticMeshComponent false (Math|Transform|MakeTransform (+ (* (Math|Vector|MakeVector (Math|Conversions|ToFloat(Integer) (.X (Utilities|Struct|BreakIntVector (Class|Block|GetLocalCoordinate _array_index)))) (Math|Conversions|ToFloat(Integer) (.Y (Utilities|Struct|BreakIntVector (Class|Block|GetLocalCoordinate _array_index)))) (Math|Conversions|ToFloat(Integer) (.Z (Utilities|Struct|BreakIntVector (Class|Block|GetLocalCoordinate _array_index))))) _tilesize) "0, 0,200.000000") "0, 0, 0" (- (/ _tilesize 1e+02) "0.200000,0.200000,0.200000"))))))
          (:then_1
            (Transformation|SetRelativeTransform (Variables|Default|GetSurroundBox) (Math|Transform|MakeTransform (* (Math|Vector|MakeVector (- (Math|Conversions|ToFloat(Integer) _x) 1.0) (- (Math|Conversions|ToFloat(Integer) _y) 1.0) (- (Math|Conversions|ToFloat(Integer) _z) 0.0)) (/ _tilesize_2 2.0)) "0, 0, 0" (Math|Vector|MakeVector (Math|Conversions|ToFloat(Integer) _x) (Math|Conversions|ToFloat(Integer) _y) (Math|Conversions|ToFloat(Integer) _z))) false false)))))))

(fn SetupPortals
  (bind _m_blockdata (Variables|Default|Getm_BlockData))
  (bind (_portalarray _tilecount) (Utilities|Struct|BreakBlockData _m_blockdata))
  (bind (_x _y _z) (Utilities|Struct|BreakIntVector _tilecount))
  (for _array_element _portalarray
    (bind _returnvalue (AddComponent|AddChildActorComponent false (Math|Transform|MakeTransform (* (Math|Vector|MakeVector (Math|Conversions|ToFloat(Integer) (Math|Integer|Clamp(Integer) (.X (Utilities|Struct|BreakIntVector (.Location (Utilities|Struct|BreakPortalData _array_element)))) 0 (- _x 1))) (Math|Conversions|ToFloat(Integer) (Math|Integer|Clamp(Integer) (.Y (Utilities|Struct|BreakIntVector (.Location (Utilities|Struct|BreakPortalData _array_element)))) 0 (- _y 1))) (Math|Conversions|ToFloat(Integer) (Math|Integer|Clamp(Integer) (.Z (Utilities|Struct|BreakIntVector (.Location (Utilities|Struct|BreakPortalData _array_element)))) 0 (- _z 1)))) 200) (Math|Rotator|MakeRotator 0.0 0.0 (* (Math|Conversions|ToInteger(Byte) (.Direction (Utilities|Struct|BreakPortalData _array_element))) 9e+01)))))
    (if (or (.IsPortal (Utilities|Struct|BreakPortalData _array_element)) (Variables|Block|GetForcePortals))
      (ChildActorComponent|SetChildActorClass _returnvalue (.PortalType (Utilities|Struct|BreakPortalData _array_element)))
      (else
        (ChildActorComponent|SetChildActorClass _returnvalue (.WallType (Utilities|Struct|BreakPortalData _array_element)))))))