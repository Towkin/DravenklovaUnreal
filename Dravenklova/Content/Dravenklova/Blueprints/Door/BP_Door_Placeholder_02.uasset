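; Placeholder interactable door with Closed, Peek and Open states, where a quick tap and a hold trigger different swings.
; A 0.25-second window separates them: tapping toggles closed/open quickly or closes from peek, while holding moves closed to peek, peek to open, or open slowly to closed.
; Timelines sweep-rotate the Anchor, update DoorState on finish, and a switching flag blocks overlapping moves.
; The construction script poses the door from its initial DoorState.
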(event EventRecieveInteractBegin
  (params (User :type D%20Character%20Object%20Reference))
  (Variables|Default|SetCurrentlyUsing true)
  (Variables|Default|SetFastSwitch true)
  (Utilities|FlowControl|Delay 0.25)
  (Variables|Default|SetFastSwitch false)
  (if (not (Variables|Default|GetCurrentlySwitching))
    (Variables|Default|SetCurrentlySwitching true)
    (switch Utilities|FlowControl|Switch|SwitchonEDoorState (Variables|Default|GetDoorState)
      (:NewEnumerator0
        (if (Variables|Default|GetFastSwitch)
          ;[1 1 1] Closed -> Open and Open -> Closed (Fast)
          (bind (_direction _closedopen) (Timeline|DoorClosedOpenFastTimeline PlayFromStart)
            (:Update
              (Transformation|SetRelativeRotation (Variables|Default|GetAnchor) (Math|Rotator|Lerp(Rotator) (Variables|Default|GetClosedRotation) (Variables|Default|GetOpenRotation) _closedopen) true false))
            (:Finished
              (Variables|Default|SetCurrentlySwitching false)
              (Variables|Default|SetCurrentlyUsing false)
              (switch Utilities|FlowControl|Switch|SwitchonETimelineDirection _direction
                (:Forward
                  (Variables|Default|SetDoorState "NewEnumerator2"))
                (:Backward
                  (Variables|Default|SetDoorState "NewEnumerator0")))))
          (else
            ;[1 1 1] Closed -> Peek and Peek -> Closed
            (bind (_direction_2 _closedpeek) (Timeline|DoorClosedPeekTimeline PlayFromStart)
              (:Update
                (Transformation|SetRelativeRotation (Variables|Default|GetAnchor) (Math|Rotator|Lerp(Rotator) (Variables|Default|GetClosedRotation) (Variables|Default|GetPeekRotation) _closedpeek) true false))
              (:Finished
                (Variables|Default|SetCurrentlySwitching false)
                (Variables|Default|SetCurrentlyUsing false)
                (switch Utilities|FlowControl|Switch|SwitchonETimelineDirection _direction_2
                  (:Forward
                    (Variables|Default|SetDoorState "NewEnumerator1"))
                  (:Backward
                    (Variables|Default|SetDoorState "NewEnumerator0"))))))))
      (:NewEnumerator1
        (if (Variables|Default|GetFastSwitch)
          (Timeline|DoorClosedPeekTimeline ReverseFromEnd)
          (else
            ;[1 1 1] Peek -> Open
            (bind _peekopen (Timeline|DoorPeekOpenTimeline PlayFromStart)
              (:Update
                (Transformation|SetRelativeRotation (Variables|Default|GetAnchor) (Math|Rotator|Lerp(Rotator) (Variables|Default|GetPeekRotation) (Variables|Default|GetOpenRotation) _peekopen) true false))
              (:Finished
                (Variables|Default|SetCurrentlySwitching false)
                (Variables|Default|SetCurrentlyUsing false)
                (Variables|Default|SetDoorState "NewEnumerator2"))))))
      (:NewEnumerator2
        (if (Variables|Default|GetFastSwitch)
          (Timeline|DoorClosedOpenFastTimeline ReverseFromEnd)
          (else
            ;[1 1 1] Closed -> Open and Open -> Closed (Slow)
            (bind (_direction_3 _closedopen_2) (Timeline|DoorClosedOpenSlow ReverseFromEnd)
              (:Update
                (Transformation|SetRelativeRotation (Variables|Default|GetAnchor) (Math|Rotator|Lerp(Rotator) (Variables|Default|GetClosedRotation) (Variables|Default|GetOpenRotation) _closedopen_2) true false))
              (:Finished
                (Variables|Default|SetCurrentlySwitching false)
                (Variables|Default|SetCurrentlyUsing false)
                (switch Utilities|FlowControl|Switch|SwitchonETimelineDirection _direction_3
                  (:Forward
                    (Variables|Default|SetDoorState "NewEnumerator2"))
                  (:Backward
                    (Variables|Default|SetDoorState "NewEnumerator0")))))))))))

(event EventRecieveInteractEnd
  (params (User :type D%20Character%20Object%20Reference))
  (if (Variables|Default|GetCurrentlyUsing)
    (Variables|Default|SetCurrentlyUsing false)
    (Utilities|FlowControl|Sequence
      (:then_1
        (if (not (Variables|Default|GetCurrentlySwitching))
          (Variables|Default|SetCurrentlySwitching true)
          (switch Utilities|FlowControl|Switch|SwitchonEDoorState (Variables|Default|GetDoorState)
            (:NewEnumerator0
              (if (Variables|Default|GetFastSwitch)
                ;[1 1 1] Closed -> Open and Open -> Closed (Fast)
                (bind (_direction _closedopen) (Timeline|DoorClosedOpenFastTimeline PlayFromStart)
                  (:Update
                    (Transformation|SetRelativeRotation (Variables|Default|GetAnchor) (Math|Rotator|Lerp(Rotator) (Variables|Default|GetClosedRotation) (Variables|Default|GetOpenRotation) _closedopen) true false))
                  (:Finished
                    (Variables|Default|SetCurrentlySwitching false)
                    (Variables|Default|SetCurrentlyUsing false)
                    (switch Utilities|FlowControl|Switch|SwitchonETimelineDirection _direction
                      (:Forward
                        (Variables|Default|SetDoorState "NewEnumerator2"))
                      (:Backward
                        (Variables|Default|SetDoorState "NewEnumerator0")))))
                (else
                  ;[1 1 1] Closed -> Peek and Peek -> Closed
                  (bind (_direction_2 _closedpeek) (Timeline|DoorClosedPeekTimeline PlayFromStart)
                    (:Update
                      (Transformation|SetRelativeRotation (Variables|Default|GetAnchor) (Math|Rotator|Lerp(Rotator) (Variables|Default|GetClosedRotation) (Variables|Default|GetPeekRotation) _closedpeek) true false))
                    (:Finished
                      (Variables|Default|SetCurrentlySwitching false)
                      (Variables|Default|SetCurrentlyUsing false)
                      (switch Utilities|FlowControl|Switch|SwitchonETimelineDirection _direction_2
                        (:Forward
                          (Variables|Default|SetDoorState "NewEnumerator1"))
                        (:Backward
                          (Variables|Default|SetDoorState "NewEnumerator0"))))))))
            (:NewEnumerator1
              (if (Variables|Default|GetFastSwitch)
                (Timeline|DoorClosedPeekTimeline ReverseFromEnd)
                (else
                  ;[1 1 1] Peek -> Open
                  (bind _peekopen (Timeline|DoorPeekOpenTimeline PlayFromStart)
                    (:Update
                      (Transformation|SetRelativeRotation (Variables|Default|GetAnchor) (Math|Rotator|Lerp(Rotator) (Variables|Default|GetPeekRotation) (Variables|Default|GetOpenRotation) _peekopen) true false))
                    (:Finished
                      (Variables|Default|SetCurrentlySwitching false)
                      (Variables|Default|SetCurrentlyUsing false)
                      (Variables|Default|SetDoorState "NewEnumerator2"))))))
            (:NewEnumerator2
              (if (Variables|Default|GetFastSwitch)
                (Timeline|DoorClosedOpenFastTimeline ReverseFromEnd)
                (else
                  ;[1 1 1] Closed -> Open and Open -> Closed (Slow)
                  (bind (_direction_3 _closedopen_2) (Timeline|DoorClosedOpenSlow ReverseFromEnd)
                    (:Update
                      (Transformation|SetRelativeRotation (Variables|Default|GetAnchor) (Math|Rotator|Lerp(Rotator) (Variables|Default|GetClosedRotation) (Variables|Default|GetOpenRotation) _closedopen_2) true false))
                    (:Finished
                      (Variables|Default|SetCurrentlySwitching false)
                      (Variables|Default|SetCurrentlyUsing false)
                      (switch Utilities|FlowControl|Switch|SwitchonETimelineDirection _direction_3
                        (:Forward
                          (Variables|Default|SetDoorState "NewEnumerator2"))
                        (:Backward
                          (Variables|Default|SetDoorState "NewEnumerator0"))))))))))))))

(fn ConstructionScript
  (bind _anchor (Variables|Default|GetAnchor))
  (switch Utilities|FlowControl|Switch|SwitchonEDoorState (Variables|Default|GetDoorState)
    (:NewEnumerator0
      (Transformation|SetRelativeRotation _anchor (Variables|Default|GetClosedRotation) false false))
    (:NewEnumerator1
      (Transformation|SetRelativeRotation _anchor (Variables|Default|GetPeekRotation) false false))
    (:NewEnumerator2
      (Transformation|SetRelativeRotation _anchor (Variables|Default|GetOpenRotation) false false))))