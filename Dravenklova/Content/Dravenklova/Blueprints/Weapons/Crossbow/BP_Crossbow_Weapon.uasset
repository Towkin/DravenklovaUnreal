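; Crossbow weapon Blueprint that stores picked-up bolts, loads one at a time and launches it as a physics projectile.
; PickupBolt stacks bolts on the weapon, and Reload moves the top one to the socketed loading point.
; Fire detaches it and applies a forward impulse, returning true even when empty.
; Equipping shows the skeletal mesh, while unequipping swaps to a physics-simulated static mesh.
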(event EventOnPrimaryActionBegin
  (bind _fired (CallFunction|Fire))
  (Variables|Default|SetIsFiring _fired)
  (Utilities|FlowControl|Delay 0.05)
  (Variables|Default|SetIsFiring false))

(event EventEquipped
  (params (User :type D%20Character%20Object%20Reference))
  (bind _staticcrossbow (Variables|Default|GetStaticCrossbow))
  (Variables|Default|SetUser User)
  (Rendering|SetVisibility (Variables|Default|GetSkeletalCrossbow) true true)
  (Rendering|SetVisibility _staticcrossbow false true)
  (Physics|SetSimulatePhysics _staticcrossbow false)
  (Collision|SetCollisionEnabled _staticcrossbow "NoCollision"))

(event EventUnequipped
  (params (User :type D%20Character%20Object%20Reference))
  (bind _staticcrossbow (Variables|Default|GetStaticCrossbow))
  (Variables|Default|SetUser 0)
  (Rendering|SetVisibility (Variables|Default|GetSkeletalCrossbow) false true)
  (Rendering|SetVisibility _staticcrossbow true true)
  (Collision|SetCollisionEnabled _staticcrossbow "QueryAndPhysics")
  (Physics|SetSimulatePhysics _staticcrossbow true)
  (Transformation|ResetRelativeTransform _staticcrossbow))

(event EventOnPrimaryActionEnd)

(event EventOnReloadActionEnd
  (Variables|Default|SetIsReloading false))

(event EventBeginPlay
  (Transformation|AttachComponentToComponent (Variables|Default|GetLoadedBoltLocation) (Variables|Default|GetSkeletalCrossbow) "Attach_Bolt_Here" "SnapToTarget" "SnapToTarget" "SnapToTarget" true))

(event EventOnReloadActionBegin
  (CallFunction|Reload)
  (Variables|Default|SetIsReloading true))

(fn ConstructionScript)

(fn PickupBolt
  (params (NewBolt :type BP%20Crossbow%20Bolt%20Object%20Reference))
  (bind _bolts (Variables|Default|GetBolts))
  (bind _capsule (Variables|/Game/Dravenklova/Blueprints/Weapons/Crossbow/BP_CrossbowBolt.BP_CrossbowBolt_C|GetCapsule NewBolt))
  (if (== (Utilities|Array|FindItem _bolts NewBolt) -1)
    (bind _returnvalue (Utilities|Array|Add _bolts NewBolt))
    (Transformation|AttachComponentToComponent NewBolt (Variables|Default|GetBoltStackLocation) "None" "SnapToTarget" "SnapToTarget" "KeepRelative" true)
    (Transformation|SetActorRelativeLocation NewBolt (* "-5.000000, 0,0.000000" (Math|Conversions|ToFloat(Integer) _returnvalue)))
    (Collision|SetActorEnableCollision NewBolt false)
    (Physics|SetSimulatePhysics _capsule false)
    (Transformation|AttachComponentToComponent _capsule (Variables|/Game/Dravenklova/Blueprints/Weapons/Crossbow/BP_CrossbowBolt.BP_CrossbowBolt_C|GetScene NewBolt) "None" "SnapToTarget" "SnapToTarget" "SnapToTarget" true)
    (Transformation|SetRelativeTransform _capsule (Variables|/Game/Dravenklova/Blueprints/Weapons/Crossbow/BP_CrossbowBolt.BP_CrossbowBolt_C|GetRelativeTransform NewBolt) false false)))

(fn TakeTopBolt
  (bind _bolts (Variables|Default|GetBolts))
  (bind _returnvalue (Utilities|Array|LastIndex _bolts))
  (if (> (Utilities|Array|Length _bolts) 0)
    (LocalVariables|SetReturnBolt (Utilities|Array|Get(acopy) _bolts _returnvalue))
    (Utilities|Array|RemoveIndex _bolts _returnvalue))
  (return (LocalVariables|GetReturnBolt)))

(fn Reload
  (if (== (Variables|Default|GetLoadedBolt) 0)
    (bind _topbolt (CallFunction|TakeTopBolt))
    (if (!= _topbolt 0)
      (bind _output_get (Variables|Default|SetLoadedBolt _topbolt))
      (Transformation|AttachComponentToComponent _output_get (Variables|Default|GetLoadedBoltLocation) "None" "SnapToTarget" "SnapToTarget" "KeepRelative" true))))

(fn Fire
  (if (!= (Variables|Default|GetLoadedBolt) 0)
    (Transformation|DetachFromActor (Variables|Default|GetLoadedBolt) "KeepRelative" "KeepRelative" "KeepRelative")
    (Physics|SetSimulatePhysics (Variables|/Game/Dravenklova/Blueprints/Weapons/Crossbow/BP_CrossbowBolt.BP_CrossbowBolt_C|GetCapsule (Variables|Default|GetLoadedBolt)) true)
    (Collision|SetActorEnableCollision (Variables|Default|GetLoadedBolt) true)
    (Physics|AddImpulse (Variables|/Game/Dravenklova/Blueprints/Weapons/Crossbow/BP_CrossbowBolt.BP_CrossbowBolt_C|GetCapsule (Variables|Default|GetLoadedBolt)) (* (Math|Vector|GetForwardVector (Variables|Default|GetLoadedBoltLocation)) 1.8e+03) "None" false)
    (Variables|Default|SetLoadedBolt 0)
    (return true)
    (else
      (return true))))