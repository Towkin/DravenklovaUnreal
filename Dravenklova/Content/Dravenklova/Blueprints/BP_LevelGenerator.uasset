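; BP_LevelGenerator is a level generator Blueprint whose BeginPlay and construction script are empty.
; An unconnected graph fragment appears to visualize the occupation grid: after a short delay, it adds a cube mesh component for every false cell.
; It converts each flat index to grid coordinates, scales them to cell size, and transforms them by the actor's transform.
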(event EventBeginPlay)

(fn ConstructionScript)