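; BP_DumLampa is a simple lamp actor whose point light is switched by things overlapping its box trigger.
; Begin and end overlap events raise and lower a counter, and the light is visible while that counter is above zero.
; The construction script derives the light's hue from the actor's world X position, so lamps placed along that axis cycle through fully saturated colors.
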(event OnComponentBeginOverlap(Box)
  (params (OverlappedComponent :type Primitive%20Component%20Object%20Reference) (OtherActor :type Actor%20Object%20Reference) (OtherComp :type Primitive%20Component%20Object%20Reference) (OtherBodyIndex :type Integer) (bFromSweep :type Boolean) (SweepResult :type Hit%20Result%20Structure%20%28by%20ref%29))
  (bind _counter (Variables|Default|GetCounter))
  (Math|Integer|IncrementInt _counter
    (:%20%20
      (Rendering|SetVisibility (Variables|Default|GetPointLight) (> _counter 0) false))))

(event OnComponentEndOverlap(Box)
  (params (OverlappedComponent :type Primitive%20Component%20Object%20Reference) (OtherActor :type Actor%20Object%20Reference) (OtherComp :type Primitive%20Component%20Object%20Reference) (OtherBodyIndex :type Integer))
  (bind _counter (Variables|Default|GetCounter))
  (Math|Integer|DecrementInt _counter
    (:%20%20
      (Rendering|SetVisibility (Variables|Default|GetPointLight) (> _counter 0) false))))

(fn ConstructionScript
  (Rendering|Components|Light|SetLightColor (Variables|Default|GetPointLight) (Class|KismetMathLibrary|HSVtoRGB (Math|Float|%(Float) (/ (.X (Math|Vector|BreakVector (Transformation|GetActorLocation))) 1e+01) 3.6e+02) 1.0 1.0 1.0) true))