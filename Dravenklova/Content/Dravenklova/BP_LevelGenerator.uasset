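; Level generator actor that visualizes its occupation grid with cube meshes at runtime.
; Shortly after BeginPlay, it loops through the grid and adds a static mesh component for every cell whose value is false.
; Each flat index is converted to 3D grid coordinates, scaled to the cell size (taller in Z) and passed through the actor transform to place the cube.
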(event EventBeginPlay
  (Utilities|FlowControl|Delay 0.2)
  (for (_array_element _array_index) (Variables|Default|Getm_OccupationGrid)
    (if (not _array_element)
      (bind _returnvalue (Class|DLevelGenerator|GlobalIndextoGrid _array_index))
      (bind _returnvalue_2 (AddComponent|AddStaticMeshComponent false (Math|Conversions|ToTransform(Vector) (Math|Transform|TransformLocation (Transformation|GetActorTransform) (Math|Vector|MakeVector (* (.X (Utilities|Struct|BreakIntVector _returnvalue)) 2e+02) (* (.Y (Utilities|Struct|BreakIntVector _returnvalue)) 2e+02) (* (.Z (Utilities|Struct|BreakIntVector _returnvalue)) 3e+02))))))
      (Components|StaticMesh|SetStaticMesh _returnvalue_2 "/Engine/BasicShapes/Cube.Cube"))))

(event Collision|EventActorBeginOverlap
  (params (OtherActor :type Actor%20Object%20Reference)))

(event EventTick
  (params (DeltaSeconds :type Float%20%28single-precision%29)))

(fn ConstructionScript)